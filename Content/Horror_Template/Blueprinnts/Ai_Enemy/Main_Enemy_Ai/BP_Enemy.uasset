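; BP_Enemy is the horror enemy that jumpscares the player on contact and ends the game.
; Its Sphere overlap toggles the player mesh's visibility, then through a DoOnce disables input and fires the Jumpscare event.
; Jumpscare cuts the view to the enemy's camera with a sound and animation, then blends back to the player.
; It then shows the WBP_Game_Over widget and, after a delay, switches to cursor-driven UI-only input.
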(event `self.Sphere.OnComponentBeginOverlap`
  (params (OverlappedComponent :type "PrimitiveComponent Object Reference") (OtherActor :type "Actor Object Reference") (OtherComp :type "PrimitiveComponent Object Reference") (OtherBodyIndex :type Integer) (bFromSweep :type Boolean) (SweepResult :type "HitResult Structure (by ref)"))
  (bind _asbp_third_person_character (cast `/Game/ThirdPerson/Blueprints/BP_ThirdPersonCharacter` OtherActor))
  (`SceneComponent.ToggleVisibility` (`Character.Mesh` _asbp_third_person_character) true)
  (`/Engine/EditorBlueprintResources/StandardMacros.DoOnce` false
    (:`Completed`
      (`self.DisableInput` (`GameplayStatics.GetPlayerCharacter` 0) (`GameplayStatics.GetPlayerController` 0))
      (`self.Jumpscare`))))

(event `Jumpscare`
  (bind _returnvalue (`GameplayStatics.GetPlayerController` 0))
  (bind _returnvalue_2 (`GameplayStatics.GetPlayerController` 0))
  (bind _returnvalue_3 (`GameplayStatics.GetPlayerCharacter` 0))
  (`PlayerController.SetViewTargetWithBlend` (`GameplayStatics.GetPlayerController` 0) (`ActorComponent.GetOwner` (`self.Camera`)) 0.0 "VTBlend_Linear" 0.0 false)
  (`GameplayStatics.PlaySound2D` "/Engine/EditorSounds/GamePreview/StartPlayInEditor.StartPlayInEditor" 1.0 1.0 0.0 null null)
  (`SkeletalMeshComponent.PlayAnimation` (`self.Mesh`) "/Game/Characters/Enemy/animations/jumpscare.jumpscare" false)
  (`KismetSystemLibrary.Delay` 1.0)
  (`PlayerController.SetViewTargetWithBlend` _returnvalue_2 _returnvalue_3 5.0 "VTBlend_Linear" 0.0 false)
  (`self.DisableInput` _returnvalue_3 _returnvalue_2)
  (`GameplayStatics.GetActorOfClass` null)
  (bind _returnvalue_4 (`|CreateWidget` "/Game/Horror_Template/UI/Game_Over/WBP_Game_Over.WBP_Game_Over_C"))
  (bind _output_get (set `self.GameOverUI` _returnvalue_4))
  (`UserWidget.AddToViewport` _output_get 0)
  (`KismetSystemLibrary.Delay` 3.0)
  (set `PlayerController.bShowMouseCursor` true _returnvalue)
  (`WidgetBlueprintLibrary.SetInputMode_UIOnlyEx` _returnvalue (`self.GameOverUI`)))

(fn `UserConstructionScript`)
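; Key-gated hinged door that swings open away from the player when interacted with, or prints that it is locked.
; Front and back overlap volumes record the player's side, choosing the ±90° yaw a timeline lerps the hinge to.
; A FlipFlop alternates open and close, but every use needs HasKey, which the timeline update clears.
; IsLocked and IsDoorMoving checks exist but are disconnected, so they never run.
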(event `self.Interactable`
  (bind _returnvalue (`GameplayStatics.GetPlayerCharacter` 0))
  (bind _asbp_third_person_character (cast `/Game/ThirdPerson/Blueprints/BP_ThirdPersonCharacter` _returnvalue))
  (if (`/Game/ThirdPerson/Blueprints/BP_ThirdPersonCharacter.HasKey?` _asbp_third_person_character)
    (set `self.IsDoorMoving?` true)
    (if (not (`self.Dooropen?`))
      (set `self.TargetRotationYaw` (`KismetMathLibrary.SelectFloat` -90.0 90.0 (`self.PlayerFrontSide?`))))
    (`/Engine/EditorBlueprintResources/StandardMacros.FlipFlop`
      (:`A`
        (bind (_direction _open_close) (`Timeline|Door Open/Close` :!label _label)
          (:`Update`
            (`SceneComponent.K2_SetRelativeRotation` (`self.DoorHinge`) (`KismetMathLibrary.MakeRotator` 0.0 0.0 (`KismetMathLibrary.Lerp` 0.0 (`self.TargetRotationYaw`) _open_close)) false false)
            (bind _asbp_third_person_character_2 (cast `/Game/ThirdPerson/Blueprints/BP_ThirdPersonCharacter` _returnvalue))
            (set `/Game/ThirdPerson/Blueprints/BP_ThirdPersonCharacter.HasKey?` false _asbp_third_person_character_2))
          (:`Finished`
            (set `self.Dooropen?` (not (`self.Dooropen?`)))
            (set `self.IsDoorMoving?` false))))
      (:`B`
        (goto _label :!via `ReverseFromEnd`)))
    (else
      (`KismetSystemLibrary.PrintString` "Door is locked"))))

(event `self.Collision_Front.OnComponentBeginOverlap`
  (params (OverlappedComponent :type "PrimitiveComponent Object Reference") (OtherActor :type "Actor Object Reference") (OtherComp :type "PrimitiveComponent Object Reference") (OtherBodyIndex :type Integer) (bFromSweep :type Boolean) (SweepResult :type "HitResult Structure (by ref)"))
  (set `self.PlayerFrontSide?` true)
  (bind _asbp_third_person_character (cast `/Game/ThirdPerson/Blueprints/BP_ThirdPersonCharacter` OtherActor))
  (set `self.Player` _asbp_third_person_character))

(event `self.Collision_Back.OnComponentBeginOverlap`
  (params (OverlappedComponent :type "PrimitiveComponent Object Reference") (OtherActor :type "Actor Object Reference") (OtherComp :type "PrimitiveComponent Object Reference") (OtherBodyIndex :type Integer) (bFromSweep :type Boolean) (SweepResult :type "HitResult Structure (by ref)"))
  (set `self.PlayerFrontSide?` false)
  (bind _asbp_third_person_character (cast `/Game/ThirdPerson/Blueprints/BP_ThirdPersonCharacter` OtherActor))
  (set `self.Player` _asbp_third_person_character))

(fn `UserConstructionScript`)